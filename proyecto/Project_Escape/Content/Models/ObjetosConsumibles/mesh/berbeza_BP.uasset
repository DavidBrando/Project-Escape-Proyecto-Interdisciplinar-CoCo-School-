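; Consumable pickup Blueprint that heals the player on touch.
; When the player character enters the Sphere overlap, a DoOnce calls Curarse on Jugador with VidaACurar, which the construction script sets.
; It then spawns the Curazion particle effect at the sphere and destroys the actor after a short delay.
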(event OnComponentBeginOverlap(Sphere)
  (params (OverlappedComponent :type Primitive%20Component%20Object%20Reference) (OtherActor :type Actor%20Object%20Reference) (OtherComp :type Primitive%20Component%20Object%20Reference) (OtherBodyIndex :type Integer) (bFromSweep :type Boolean) (SweepResult :type Hit%20Result%20Structure%20%28by%20ref%29))
  (if (== OtherActor (Game|GetPlayerCharacter 0))
    (bind _asjugador (Utilities|Casting|CastToJugador OtherActor))
    (Utilities|FlowControl|DoOnce false
      (:Completed
        (Default|Curarse _asjugador (Variables|Default|GetvidaACurar))
        (Effects|SpawnEmitteratLocation "/Game/Models/ObjetosConsumibles/curazion.curazion" (Transformation|GetWorldLocation (Variables|Default|GetSphere)))
        (Utilities|FlowControl|Delay 0.2)
        (Actor|DestroyActor)))))

(event EventBeginPlay)

(event Collision|EventActorBeginOverlap
  (params (OtherActor :type Actor%20Object%20Reference)))

(event EventTick
  (params (DeltaSeconds :type Float%20%28single-precision%29)))

(fn ConstructionScript
  (Variables|Default|SetvidaACurar 2e+01))